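; Wooden arrow ammunition item for the Pixel2D game, stored as a stackable piece of equipment.
; When used, it reduces its equipment stack by one.
; GetAmmoStats exposes its ammo type, projectile class and bonus damage, knockback and speed from variables.
; BeginPlay, overlap and Tick are disabled stubs, and the construction script only calls the parent.
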(event EventBeginPlay
  (|CallParentFunction) ; This node is disabled and will not be called.\nDrag off pins to build functionality.
)

(event Collision|EventActorBeginOverlap
  (params (OtherActor :type Actor%20Object%20Reference))
  (|CallParentFunction OtherActor) ; This node is disabled and will not be called.\nDrag off pins to build functionality.
)

(event EventTick
  (params (DeltaSeconds :type Float%20%28single-precision%29))
  (|CallParentFunction DeltaSeconds) ; This node is disabled and will not be called.\nDrag off pins to build functionality.
)

(event EventOnUsed
  (params (OwningActor :type Actor%20Object%20Reference))
  (CallFunction|DecreaseEquipmentStack 1))

(fn ConstructionScript
  (|CallParentFunction))

(fn GetAmmoStats
  (return (Variables|Default|GetammoType) (Variables|Default|GetprojectileClass) (Variables|Default|GetdDamageBonus) (Variables|Default|GetknockbackBonus) (Variables|Default|GetspeedBonus)))