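; Demo Blueprint for a destroyable 2D tilemap that randomly breaks itself apart when its OnHit event fires.
; Each pass calls HideActorTile on itself for three random cells within an 8x8 area, rebuilding collision on every call.
; A DoN node and a very short Delay loop the pass up to 500 times, and the counter is never reset.
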(event Custom|caca)

(event EventBeginPlay
  (|CallParentFunction) ; This node is disabled and will not be called.\nDrag off pins to build functionality.
)

(event Collision|EventActorBeginOverlap
  (params (OtherActor :type Actor%20Object%20Reference))
  (|CallParentFunction OtherActor) ; This node is disabled and will not be called.\nDrag off pins to build functionality.
)

(event EventTick
  (params (DeltaSeconds :type Float%20%28single-precision%29))
  (|CallParentFunction DeltaSeconds) ; This node is disabled and will not be called.\nDrag off pins to build functionality.
)

(event EventOnHit
  (CallFunction|HideActorTile self 0 (Math|Random|RandomIntegerinRange 0 7) (Math|Random|RandomIntegerinRange 0 7) true :!label _label)
  (CallFunction|HideActorTile self 0 (Math|Random|RandomIntegerinRange 0 7) (Math|Random|RandomIntegerinRange 0 7) true)
  (CallFunction|HideActorTile self 0 (Math|Random|RandomIntegerinRange 0 7) (Math|Random|RandomIntegerinRange 0 7) true)
  (Utilities|FlowControl|DoN 500
    (:Exit
      (Utilities|FlowControl|Delay 0.001)
      (goto _label))))

(fn ConstructionScript
  (|CallParentFunction))