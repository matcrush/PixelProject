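; Actor component that damages an actor's BP_HealthComponent, with knockback, through externally called DealDamage and StopDealingDamage events.
; Each successful hit spawns red floating combat text showing the damage amount.
; Knockback combines the hit normal with a configured force.
; With a positive DamageFrequency, a Delay loop repeats damage until a single shared flag, not tracked per actor, is cleared.
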(event Custom|DealDamage
  (params (DamagedActor :type Actor%20Object%20Reference) (HitNormal :type Vector))
  (bind _returnvalue (Actor|GetComponentbyClass DamagedActor "/Game/Pixel2D/Blueprints/Components/BP_HealthComponent.BP_HealthComponent_C"))
  (bind _damageamount (Variables|Default|GetdamageAmount))
  (bind _damagefrequency (Variables|Default|GetdamageFrequency))
  (Variables|Default|SetisDealingDamage true)
  (if (Variables|Default|GetisDealingDamage) :!label _label
    (Utilities|IsValid _returnvalue
      (:Is%20Valid
        (bind _result (Default|DecreaseHealth _returnvalue _damageamount (CallFunction|NormalizedMultiplication HitNormal (Variables|Default|GetknockbackForce)) (Components|GetOwner)))
        (if _result
          (CallFunction|SpawnFloatingCombatText "NewEnumerator0" (Utilities|Text|ToText(Integer) _damageamount) 0 (Transformation|GetActorLocation DamagedActor) "(R=1.000000,G=0.000000,B=0.067033,A=1.000000)"))
        (if (> _damagefrequency 0.0)
          (Utilities|FlowControl|Delay _damagefrequency)
          (goto _label))))))

(event Custom|StopDealingDamage
  (params (DamagedActor :type Actor%20Object%20Reference))
  (Variables|Default|SetisDealingDamage false))

(event EventBeginPlay)

(event EventTick
  (params (DeltaSeconds :type Float%20%28single-precision%29)))